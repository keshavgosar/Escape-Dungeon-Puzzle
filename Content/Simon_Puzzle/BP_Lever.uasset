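; BP_Lever is an interactable on/off lever actor in the Simon puzzle folder.
; DisplayUI writes the "Press E" interaction prompt to the first-person character's HUD.
; Interact toggles IsOn and plays the Rotate timeline, easing the lever mesh's pitch between two angles while a flag blocks re-triggering.
; When the timeline finishes, it swaps the start and end angles, so the next interaction swings the lever back.
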(event `/Game/BPI_Interact.DisplayUI`
  (params (IsStorageUnlocked :type Boolean))
  ; Display Prompt logic
  (bind _asbp_first_person_character (cast `/Game/FirstPerson/Blueprints/BP_FirstPersonCharacter` (`GameplayStatics.GetPlayerPawn` 0)))
  (bind _playerhud (`EscapeTimeLoopCharacter.PlayerHUD` _asbp_first_person_character))
  (`/Engine/EditorBlueprintResources/StandardMacros.IsValid` _playerhud
    (:`Is Valid`
      (set `TextBlock.Text` "Press \"E\" to interact" (`PlayerHUD.PromptDisplay` _playerhud)))))

(event `/Game/BPI_Interact.Interact`
  ; Lever On/Off logic
  (if (`self.HasRotationFinished`)
    (set `self.HasRotationFinished` false)
    (set `self.bIsOn` (not (`self.bIsOn`)))
    (bind (_direction _alpha) (`Timeline|Rotate` :!via `PlayFromStart`)
      (:`Update`
        (`SceneComponent.K2_SetRelativeRotation` (`self.LeverMesh`) (`KismetMathLibrary.MakeRotator` 0.0 (`|EaseFunction` "EaseInOut" _alpha (`self.LeverInitialRotationValue`) (`self.LeverFinalRotateValue`))) false false))
      (:`Finished`
        (set `self.Temp` (`self.LeverInitialRotationValue`))
        (set `self.LeverInitialRotationValue` (`self.LeverFinalRotateValue`))
        (set `self.LeverFinalRotateValue` (`self.Temp`))
        (set `self.HasRotationFinished` true)))))

(fn `UserConstructionScript`)