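; BP_Cup is a collectible cup, apparently for the Simon puzzle, that can only be taken once storage is unlocked.
; DisplayUI shows an "E" pickup prompt on the first-person character's HUD when unlocked.
; Interact adds "Cup" to the character's Inventory, then clears the prompt and destroys the actor.
; The clear and destroy depend on the character reference cast in DisplayUI and a valid prompt widget.
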(event `/Game/BPI_Interact.DisplayUI`
  (params (IsStorageUnlocked :type Boolean))
  (if IsStorageUnlocked
    (bind _asbp_first_person_character (cast `/Game/FirstPerson/Blueprints/BP_FirstPersonCharacter` (`GameplayStatics.GetPlayerPawn` 0)))
    (bind _promptdisplay (`PlayerHUD.PromptDisplay` (`EscapeTimeLoopCharacter.PlayerHUD` _asbp_first_person_character)))
    (`/Engine/EditorBlueprintResources/StandardMacros.IsValid` _promptdisplay
      (:`Is Valid`
        (`TextBlock.SetText` _promptdisplay "Press \"E\" to take the cup")))))

(event `/Game/BPI_Interact.Interact`
  (if (stale `/Game/BPI_Interact.DisplayUI` IsStorageUnlocked)
    (bind _asbp_first_person_character (cast `/Game/FirstPerson/Blueprints/BP_FirstPersonCharacter` (`GameplayStatics.GetPlayerPawn` 0)))
    (`BlueprintMapLibrary.Map_Add` (`EscapeTimeLoopCharacter.Inventory` _asbp_first_person_character) "Cup" 1)
    (bind _promptdisplay (`PlayerHUD.PromptDisplay` (`EscapeTimeLoopCharacter.PlayerHUD` (stale `/Game/BPI_Interact.DisplayUI` _asbp_first_person_character))))
    (`/Engine/EditorBlueprintResources/StandardMacros.IsValid` _promptdisplay
      (:`Is Valid`
        (`TextBlock.SetText` _promptdisplay "")
        (`self.K2_DestroyActor`)))))

(fn `UserConstructionScript`)