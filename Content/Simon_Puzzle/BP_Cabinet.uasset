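; BP_Cabinet is a puzzle cabinet that unlocks when its three child-actor levers all match their correct states.
; While the player is inside InteractStartBox, Tick line-traces from the player's view to prompt and interact with BPI_Interact actors, clearing the HUD prompt otherwise.
; After each interaction while locked, it checks the levers and, on a match, brightens the bulb and plays the door-opening animation.
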(event `self.ReceiveTick`
  (params (DeltaSeconds :type "Float (single-precision)"))
  (bind (_location _rotation) (`Controller.GetPlayerViewPoint` (`GameplayStatics.GetPlayerController` 0)))
  (if (`self.ShouldStartTrace`)
    (bind (_outhit _returnvalue) (`KismetSystemLibrary.LineTraceSingle` _location (+ _location (* (`KismetMathLibrary.GetForwardVector` _rotation) 5000.0)) "TraceTypeQuery3"))
    (if (and _returnvalue (`KismetSystemLibrary.DoesImplementInterface` (`.HitActor` (`GameplayStatics.BreakHitResult` _outhit)) "/Game/BPI_Interact.BPI_Interact_C"))
      (message `/Game/BPI_Interact.DisplayUI` (`.HitActor` (`GameplayStatics.BreakHitResult` _outhit)) (`self.IsCabinetUnlocked`))
      (bind _asbp_first_person_character (cast `/Game/FirstPerson/Blueprints/BP_FirstPersonCharacter` (`GameplayStatics.GetPlayerPawn` 0)))
      (if (`EscapeTimeLoopCharacter.bIsInteracting` _asbp_first_person_character)
        (message `/Game/BPI_Interact.Interact` (`.HitActor` (`GameplayStatics.BreakHitResult` _outhit)))
        (if (not (`self.IsCabinetUnlocked`))
          (bind _shouldunlocksafe (`self.IsCombinationCodeCorrect`))
          (if _shouldunlocksafe
            (set `self.IsCabinetUnlocked` true)
            (`LightComponent.SetIntensity` (`self.BulbLight`) 1000.0)
            (`SkeletalMeshComponent.PlayAnimation` (`self.CabinetDoorMesh`) "/Game/Animations/cabinet_door_open/cabinet_door_opening_animation_Anim.cabinet_door_opening_animation_Anim" false))))
      (else
        (`self.HideUI`)))))

(event `self.Interact Start Box.OnComponentBeginOverlap`
  (params (OverlappedComponent :type "PrimitiveComponent Object Reference") (OtherActor :type "Actor Object Reference") (OtherComp :type "PrimitiveComponent Object Reference") (OtherBodyIndex :type Integer) (bFromSweep :type Boolean) (SweepResult :type "HitResult Structure (by ref)"))
  (cast `/Game/FirstPerson/Blueprints/BP_FirstPersonCharacter` OtherActor)
  (set `self.ShouldStartTrace` true))

(event `self.Interact Start Box.OnComponentEndOverlap`
  (params (OverlappedComponent :type "PrimitiveComponent Object Reference") (OtherActor :type "Actor Object Reference") (OtherComp :type "PrimitiveComponent Object Reference") (OtherBodyIndex :type Integer))
  (set `self.ShouldStartTrace` false)
  (`self.HideUI`))

(fn `HideUI`
  (bind _asbp_first_person_character (cast `/Game/FirstPerson/Blueprints/BP_FirstPersonCharacter` (`GameplayStatics.GetPlayerPawn` 0)))
  (bind _playerhud (`EscapeTimeLoopCharacter.PlayerHUD` _asbp_first_person_character))
  (`/Engine/EditorBlueprintResources/StandardMacros.IsValid` _playerhud
    (:`Is Valid`
      (set `TextBlock.Text` "" (`PlayerHUD.PromptDisplay` _playerhud)))))

(fn `IsCombinationCodeCorrect`
  (returns (ShouldUnlockSafe :type Boolean))
  (`|ExecutionSequence`
    (:`then_0`
      (bind _asbp_lever (cast `/Game/Simon_Puzzle/BP_Lever` (`ChildActorComponent.ChildActor` (`self.LeftLever`))))
      (set `self.IsLeftLeverCorrect` (== (`Lever.bIsOn` _asbp_lever) (`Lever.bCorrectState` _asbp_lever))))
    (:`then_1`
      (bind _asbp_lever_2 (cast `/Game/Simon_Puzzle/BP_Lever` (`ChildActorComponent.ChildActor` (`self.MiddleLever`))))
      (set `self.IsMiddleLeverCorrect` (== (`Lever.bIsOn` _asbp_lever_2) (`Lever.bCorrectState` _asbp_lever_2))))
    (:`then_2`
      (bind _asbp_lever_3 (cast `/Game/Simon_Puzzle/BP_Lever` (`ChildActorComponent.ChildActor` (`self.RightLever`))))
      (set `self.IsRightLeverCorrect` (== (`Lever.bIsOn` _asbp_lever_3) (`Lever.bCorrectState` _asbp_lever_3))))
    (:`then_3`
      (return (and (and (`self.IsLeftLeverCorrect`) (`self.IsMiddleLeverCorrect`)) (`self.IsRightLeverCorrect`))))))

(fn `UserConstructionScript`)