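; BP_Chest is a locked chest that plays its lid-opening animation when the player interacts while holding a ChestKey.
; An overlap box enables a per-tick camera line trace, which sends prompt and interact messages to hit actors implementing BPI_Interact.
; DisplayUI and Interact update the player's HUD prompt and check the inventory.
; Without a key, a "Needs a Chest Key" message briefly pauses the normal prompt.
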(event `self.ReceiveTick`
  (params (DeltaSeconds :type "Float (single-precision)"))
  (bind (_location _rotation) (`Controller.GetPlayerViewPoint` (`GameplayStatics.GetPlayerController` 0)))
  (if (`self.ShouldStartTrace`)
    (bind (_outhit _returnvalue) (`KismetSystemLibrary.LineTraceSingle` :`Start` _location :`End` (+ _location (* (`KismetMathLibrary.GetForwardVector` _rotation) 5000.0)) :`TraceChannel` "TraceTypeQuery3" :`bIgnoreSelf` (`self.IsChestUnlocked`)))
    (if (and _returnvalue (`KismetSystemLibrary.DoesImplementInterface` (`.HitActor` (`GameplayStatics.BreakHitResult` _outhit)) "/Game/BPI_Interact.BPI_Interact_C"))
      (message `/Game/BPI_Interact.DisplayUI` (`.HitActor` (`GameplayStatics.BreakHitResult` _outhit)) (`self.IsChestUnlocked`))
      (bind _asbp_first_person_character (cast `/Game/FirstPerson/Blueprints/BP_FirstPersonCharacter` (`GameplayStatics.GetPlayerPawn` 0)))
      (if (`EscapeTimeLoopCharacter.bIsInteracting` _asbp_first_person_character)
        (message `/Game/BPI_Interact.Interact` (`.HitActor` (`GameplayStatics.BreakHitResult` _outhit))))
      (else
        (`self.HideUI`)))))

(event `self.Interact Start Box.OnComponentBeginOverlap`
  (params (OverlappedComponent :type "PrimitiveComponent Object Reference") (OtherActor :type "Actor Object Reference") (OtherComp :type "PrimitiveComponent Object Reference") (OtherBodyIndex :type Integer) (bFromSweep :type Boolean) (SweepResult :type "HitResult Structure (by ref)"))
  (cast `/Game/FirstPerson/Blueprints/BP_FirstPersonCharacter` OtherActor)
  (set `self.ShouldStartTrace` true))

(event `self.Interact Start Box.OnComponentEndOverlap`
  (params (OverlappedComponent :type "PrimitiveComponent Object Reference") (OtherActor :type "Actor Object Reference") (OtherComp :type "PrimitiveComponent Object Reference") (OtherBodyIndex :type Integer))
  (set `self.ShouldStartTrace` false)
  (`self.HideUI`)
  (set `self.PauseDisplay` false))

(event `/Game/BPI_Interact.DisplayUI`
  (params (IsStorageUnlocked :type Boolean))
  (if (and (not IsStorageUnlocked) (not (`self.PauseDisplay`)))
    (bind _asbp_first_person_character (cast `/Game/FirstPerson/Blueprints/BP_FirstPersonCharacter` (`GameplayStatics.GetPlayerPawn` 0)))
    (bind _promptdisplay (`PlayerHUD.PromptDisplay` (`EscapeTimeLoopCharacter.PlayerHUD` _asbp_first_person_character)))
    (`/Engine/EditorBlueprintResources/StandardMacros.IsValid` _promptdisplay
      (:`Is Valid`
        (`TextBlock.SetText` _promptdisplay "Press \"E\" to interact")))))

(event `/Game/BPI_Interact.Interact`
  (bind _chestlid (`self.ChestLid`))
  (if (not (`self.IsChestUnlocked`))
    (bind _asbp_first_person_character (cast `/Game/FirstPerson/Blueprints/BP_FirstPersonCharacter` (`GameplayStatics.GetPlayerPawn` 0)))
    (if (> (`BlueprintMapLibrary.Map_Find` (`EscapeTimeLoopCharacter.Inventory` _asbp_first_person_character) "ChestKey") 0)
      (`/Engine/EditorBlueprintResources/StandardMacros.IsValid` _chestlid
        (:`Is Valid`
          (`SkeletalMeshComponent.PlayAnimation` _chestlid "/Game/Animations/chest_opening/chest_lid_opening__Anim.chest_lid_opening__Anim" false)
          (set `self.IsChestUnlocked` true)
          (bind _promptdisplay (`PlayerHUD.PromptDisplay` (`EscapeTimeLoopCharacter.PlayerHUD` (stale `/Game/BPI_Interact.DisplayUI` _asbp_first_person_character))))
          (`/Engine/EditorBlueprintResources/StandardMacros.IsValid` _promptdisplay
            (:`Is Valid`
              (`TextBlock.SetText` _promptdisplay "")))))
      (else
        (bind _promptdisplay_2 (`PlayerHUD.PromptDisplay` (`EscapeTimeLoopCharacter.PlayerHUD` _asbp_first_person_character)))
        (`/Engine/EditorBlueprintResources/StandardMacros.IsValid` _promptdisplay_2
          (:`Is Valid`
            (`TextBlock.SetText` _promptdisplay_2 "Needs a Chest Key")
            (set `self.PauseDisplay` true)
            (`KismetSystemLibrary.Delay` 1.5)
            (`TextBlock.SetText` _promptdisplay_2 "")
            (set `self.PauseDisplay` false)))))))

(fn `HideUI`
  (bind _asbp_first_person_character (cast `/Game/FirstPerson/Blueprints/BP_FirstPersonCharacter` (`GameplayStatics.GetPlayerPawn` 0)))
  (bind _playerhud (`EscapeTimeLoopCharacter.PlayerHUD` _asbp_first_person_character))
  (`/Engine/EditorBlueprintResources/StandardMacros.IsValid` _playerhud
    (:`Is Valid`
      (set `TextBlock.Text` "" (`PlayerHUD.PromptDisplay` _playerhud)))))

(fn `UserConstructionScript`)